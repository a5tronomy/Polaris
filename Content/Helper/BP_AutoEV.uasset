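; BP_AutoEV is a helper actor that applies one exposure value, AutoEV, across the lighting and post-process actors in a level.
; Its Construction Script finds every character light controller and light sublevel param actor and copies AutoEV into their target and current EV fields.
; It also sets each battle post-process volume's min and max EV100 to AutoEV, pinning auto exposure, and its exposure compensation to AutoBias.
; The event graph is unused.
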(event EventBeginPlay)

(event Collision|EventActorBeginOverlap
  (params (OtherActor :type Actor%20Object%20Reference)))

(event EventTick
  (params (DeltaSeconds :type Float%20%28single-precision%29)))

(fn ConstructionScript
  (bind _autoev (Variables|Default|GetAutoEV))
  (bind _outactors (Actor|GetAllActorsOfClass "/Game/Blueprints/Light/BP_CharacterLightController.BP_CharacterLightController_C"))
  (for _array_element _outactors
    (bind _output_get (Variables|/Game/Blueprints/Light/BP_CharacterLightController.BP_CharacterLightController_C|SetStageEV _array_element (Variables|Default|GetAutoEV)))
    (Variables|/Game/Blueprints/Light/BP_CharacterLightController.BP_CharacterLightController_C|SetStageEV_current _array_element _output_get))
  (bind _outactors_2 (Actor|GetAllActorsOfClass "/Game/Blueprints/Light/BP_LightSublevelParam.BP_LightSublevelParam_C"))
  (for _array_element_2 _outactors_2
    (bind _output_get_2 (Variables|/Game/Blueprints/Light/BP_LightSublevelParam.BP_LightSublevelParam_C|SetEV_for_LightCorrection _array_element_2 (Variables|Default|GetAutoEV)))
    (Variables|/Game/Blueprints/Light/BP_LightSublevelParam.BP_LightSublevelParam_C|SetEV_for_LightCorrection_current _array_element_2 _output_get_2))
  (bind _outactors_3 (Actor|GetAllActorsOfClass "/Game/Stage/Common/Blueprints/BP_PolarisPostProcessVolume_Battle_Base.BP_PolarisPostProcessVolume_Battle_Base_C"))
  (for _array_element_3 _outactors_3
    (Utilities|Struct|SetmembersinPostProcessSettings (Variables|/Script/Engine.PostProcessVolume|GetSettings _array_element_3) (Variables|Default|GetAutoBias) _autoev _autoev)))