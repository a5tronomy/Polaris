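; BP_WallCleaner is a helper actor that hides the contents of one streaming level, identified by GeomLevel, when play begins.
; BeginPlay calls HideLevelAssets, which scans every actor in the world and compares its level to that streaming level's loaded level.
; Matching actors are hidden in game and have their actor tick disabled, with no change to their collision.
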(event EventBeginPlay
  (CallFunction|HideLevelAssets))

(event Collision|EventActorBeginOverlap
  (params (OtherActor :type Actor%20Object%20Reference)))

(event EventTick
  (params (DeltaSeconds :type Float%20%28single-precision%29)))

(fn ConstructionScript)

(fn HideLevelAssets
  (bind _outactors (Actor|GetAllActorsOfClass "/Script/Engine.Actor"))
  (for _array_element _outactors
    (LocalVariables|SetActor _array_element)
    (if (== (Class|Actor|GetLevel (LocalVariables|GetActor)) (Class|LevelStreaming|GetLoadedLevel (Class|GameplayStatics|GetStreamingLevel (Variables|Default|GetGeomLevel))))
      (Rendering|SetActorHiddenInGame (LocalVariables|GetActor) true)
      (Actor|Tick|SetActorTickEnabled (LocalVariables|GetActor)))))