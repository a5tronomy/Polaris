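; BP_FacadeController is a debug-stage actor that tells the materials on a set of static mesh actors which direction the controller lies from each mesh.
; On BeginPlay it creates a dynamic material instance for every material slot on each actor in SMActors and stores them in DynamicMIs.
; Each instance's FacadeVector parameter receives the normalized mesh-to-controller direction, with Z (blue channel) zeroed unless SetBCh is set.
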(event EventBeginPlay
  (for _array_element (Variables|Default|GetSM_Actors)
    (Variables|Default|SetCurrentStaticMesh (Variables|/Script/Engine.StaticMeshActor|GetStaticMeshComponent _array_element))
    (for (_array_element_2 _array_index) (Rendering|Material|GetMaterials (Variables|Default|GetCurrentStaticMesh))
      (bind _returnvalue (Rendering|Material|CreateDynamicMaterialInstance (Variables|Default|GetCurrentStaticMesh) _array_index _array_element_2 "MI_Facade" :!class /Script/Engine.PrimitiveComponent))
      (if (Variables|Default|GetSet_B_Ch)
        (Rendering|Material|SetVectorParameterValue _returnvalue "FacadeVector" (Math|Conversions|ToLinearColor(Vector) (Math|Vector|Normalize (- (Transformation|GetActorLocation) (Transformation|GetActorLocation _array_element)))) :!class /Script/Engine.MaterialInstanceDynamic)
        (else
          (Rendering|Material|SetVectorParameterValue _returnvalue "FacadeVector" (Math|Conversions|ToLinearColor(Vector) (Math|Vector|MakeVector (.X (Math|Vector|BreakVector (Math|Vector|Normalize (- (Transformation|GetActorLocation) (Transformation|GetActorLocation _array_element))))) (.Y (Math|Vector|BreakVector (Math|Vector|Normalize (- (Transformation|GetActorLocation) (Transformation|GetActorLocation _array_element))))) 0.0)) :!class /Script/Engine.MaterialInstanceDynamic)))
      (Utilities|Array|Add (Variables|Default|GetDynamicMIs) _returnvalue))))

(fn ConstructionScript)