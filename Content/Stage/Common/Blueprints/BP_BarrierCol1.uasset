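; BP_BarrierCol1 is a stage barrier actor whose Blueprint logic only drives its BarrierDirection arrow in the Construction Script.
; When wall barrier groups exist, it yaws the arrow to match the first group's FacadeVector.
; The arrow turns white if FirstBarrierVector references any actors across its mesh, gimmick, mob and other lists, and grey otherwise.
; The event graph has no active logic.
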(event EventBeginPlay)

(event Collision|EventActorBeginOverlap
  (params (OtherActor :type Actor%20Object%20Reference)))

(event EventTick
  (params (DeltaSeconds :type Float%20%28single-precision%29)))

(fn ConstructionScript
  (bind _wallbarriergroups (Variables|Default|GetWallBarrierGroups))
  (bind _firstbarriervector (LocalVariables|GetFirstBarrierVector))
  (bind (_staticmeshactors _skeletalmeshactors _stagegimmickactors _mobactors _mobanimals _reactionmob _actionvatmobactors _otheractors) (Utilities|Struct|BreakWallBarrierGroup _firstbarriervector))
  (bind _output (Utilities|Array|Get(acopy) _wallbarriergroups))
  (bind _facadevector (Utilities|Struct|BreakWallBarrierGroup _output))
  (bind (_x _y) (Math|Vector|BreakVector _facadevector))
  (|CallParentFunction)
  (if (> (Utilities|Array|Length (Variables|Default|GetWallBarrierGroups)) 0)
    (Variables|/Script/Engine.ArrowComponent|SetArrowColor (Variables|Default|GetBarrierDirection) (select (> (+ (Utilities|Array|Length _staticmeshactors) (Utilities|Array|Length _skeletalmeshactors) (Utilities|Array|Length _stagegimmickactors) (Utilities|Array|Length _mobactors) (Utilities|Array|Length _mobanimals) (Utilities|Array|Length _reactionmob) (Utilities|Array|Length _actionvatmobactors) (Utilities|Array|Length _otheractors)) 0) (Math|Color|MakeColor 255 255 255 255) (Math|Color|MakeColor 125 125 125 255)))
    (Transformation|SetWorldRotation (Variables|Default|GetBarrierDirection) (Math|Rotator|MakeRotator 0.0 0.0 (Class|KismetMathLibrary|DegAtan2 _y _x)) false false)))