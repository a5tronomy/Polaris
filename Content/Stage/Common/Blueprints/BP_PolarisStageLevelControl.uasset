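; Stage level control Blueprint that starts a level sequence when the stage begins play.
; On BeginPlay it takes the values of the BattleEventLevelSequence map and, if any exist, creates a player for the first sequence of the first entry and plays it.
; The PlaySequence and OnGeneralBattleEvent events are empty, so battle event type does not affect playback here.
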(event Custom|Play%20Sequence)

(event Custom|On%20General%20Battle%20Event
  (params (Type :type EGeneralBattleEvent%20Enum :default "None")))

(event EventBeginPlay
  (bind _values (Utilities|Map|Values (Variables|Default|GetBattleEventLevelSequence)))
  (if (> (Utilities|Array|Length _values) 0)
    (bind _outactor (Sequencer|Player|CreateLevelSequencePlayer (.LevelSequence (Utilities|Struct|BreakStageLevelSequenceAsset (Utilities|Array|Get(acopy) (.LevelSequence (Utilities|Struct|BreakStageLevelSequence (Utilities|Array|Get(acopy) _values))))))))
    (Sequencer|Player|Play (Variables|/Script/LevelSequence.LevelSequenceActor|GetSequencePlayer _outactor) :!class /Script/MovieScene.MovieSceneSequencePlayer)))

(event Collision|EventActorBeginOverlap
  (params (OtherActor :type Actor%20Object%20Reference)))

(event EventTick
  (params (DeltaSeconds :type Float%20%28single-precision%29)))

(fn ConstructionScript)